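; BP_Bomb is a timed bomb actor that bursts into projectiles along four perpendicular directions.
; On BeginPlay, a timeline animates the bomb's scale while a timer counts down to ChainReaction.
; ChainReaction spawns a BP_Projectile every 90 degrees, slightly above the bomb, with lifespan scaled by the Int event's input, then destroys the bomb.
; Ending an overlap calls the LeftBombCollision dispatcher.
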(event EventBeginPlay
  (Utilities|Time|SetTimerbyEvent (delegate EventChainReaction) 3.0)
  (bind _bombscale (Timeline|Exploding%20Timeline Play)
    (:Update
      (Transformation|SetWorldScale3D (Variables|Default|GetBomb) (Math|Conversions|ToVector(Float) _bombscale)))))

(event EventChainReaction
  (for _index (range 0 3)
    (bind _returnvalue (Game|SpawnActorfromClass "/Game/MyStuff/BP_Projectile.BP_Projectile_C" (Math|Transform|MakeTransform (+ (Transformation|GetActorLocation) "0.000000,0.000000,100.000000") (Math|Conversions|RotationFromXVector (Math|Vector|RotateVector "1.000000,0.000000,0.000000" (Math|Rotator|MakeRotator 0.0 0.0 (Math|Conversions|ToFloat(Integer) (* _index 90))))) "1.000000,1.000000,1.000000") "Undefined" "MultiplyWithRoot" 0 0))
    (Actor|SetLifeSpan _returnvalue (* (stale EventInt a) 0.133)))
  (Actor|DestroyActor))

(event EventInt
  (params (a :type Integer)))

(event Collision|EventActorEndOverlap
  (params (OtherActor :type Actor%20Object%20Reference))
  (Default|CallLeftBombCollision))

(fn ConstructionScript)