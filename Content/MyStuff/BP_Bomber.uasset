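; BP_Bomber is a Bomberman-style character that plants grid-snapped bombs on input and tracks how many are active.
; Each spawned BP_Bomb receives the current power, and the capsule ignores its blocking box until the bomb signals it was left.
; That signal restores collision and allows another bomb if under the limit, while bomb removal decrements the count and re-enables placement.
; Upgrade events raise clamped power and capacity.
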(event Custom|Clear%20Bomb%20Collision
  (Class|PrimitiveComponent|ClearMoveIgnoreComponents (Variables|Default|GetCapsuleComponent))
  (if (not (>= (Variables|Default|GetBombCount) (Variables|Default|GetBombMax)))
    (Variables|Default|SetCanPlaceBomb true)))

(event Custom|Upgrade%20Bomb%20Power
  (bind _output_get (Variables|Default|SetBombPower (Math|Integer|Clamp(Integer) (+ (Variables|Default|GetBombPower) 1) 1 6))))

(event Custom|Upgrade%20Bomb%20Max
  (Variables|Default|SetBombMax (Math|Integer|Clamp(Integer) (+ (Variables|Default|GetBombMax) 1) 1 5)))

(event Custom|RemoveBomb
  (params (Actor :type Actor%20Object%20Reference) (EndPlayReason :type EEndPlayReason%20Enum :default "Destroyed"))
  (Variables|Default|SetBombCount (- (Variables|Default|GetBombCount) 1))
  (Variables|Default|SetCanPlaceBomb true))

(event EventEndPlay
  (params (EndPlayReason :type EEndPlayReason%20Enum :default "Destroyed")))

(event Input|ActionEvents|InputActionPlantBomb
  (params (Key :type Key%20Structure :default "None"))
  (:Pressed
    (if (Variables|Default|GetCanPlaceBomb)
      (bind _returnvalue (Game|SpawnActorfromClass "/Game/MyStuff/BP_Bomb.BP_Bomb_C" (Math|Transform|MakeTransform (Class|KismetMathLibrary|VectorSnappedtoGrid (Transformation|GetActorLocation) 2e+02) "0, 0, 0" "0.700000,0.700000,0.700000") "AlwaysSpawn" "OverrideRootScale" self 0))
      (Class|BPIInteger|Int(Message) _returnvalue (stale Custom|Upgrade%20Bomb%20Power _output_get))
      (Variables|Default|SetCanPlaceBomb false)
      (Variables|Default|SetBombCount (+ (Variables|Default|GetBombCount) 1))
      (Class|PrimitiveComponent|IgnoreComponentwhenMoving (Variables|Default|GetCapsuleComponent) (Variables|/Game/MyStuff/BP_Bomb.BP_Bomb_C|GetBlockBox _returnvalue) true)
      (EventDispatchers|BindEventtoLeftBombCollision _returnvalue (delegate Custom|Clear%20Bomb%20Collision))
      (Game|BindEventtoOnEndPlay _returnvalue (delegate Custom|RemoveBomb)))))

(fn ConstructionScript)

(fn Int
  (params (a :type Integer))
  (return))