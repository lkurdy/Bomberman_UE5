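; Game mode for a Bomberman-style game that thins out the level's placed crates at startup.
; On BeginPlay it calls GenerateLevel, which gathers every BP_Crate actor and destroys randomly picked ones, removing each from the working list.
; The loop count scales with the CrateDeletion fraction, which BeginPlay currently passes as zero.
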(event EventBeginPlay
  (CallFunction|GenerateLevel 0.0))

(event EventTick
  (params (DeltaSeconds :type Float%20%28single-precision%29)))

(fn ConstructionScript)

(fn GenerateLevel
  (params (CrateDeletion%25 :type Float%20%28double-precision%29))
  (bind _outactors (Actor|GetAllActorsOfClass "/Game/MyStuff/BP_Crate.BP_Crate_C"))
  (LocalVariables|SetCrates _outactors)
  (for _index (range 0 (Math|Float|Truncate (* (Utilities|Array|Length _outactors) CrateDeletion%25)))
    (bind _output_get (LocalVariables|SetRandom%20Crate (.OutItem (Utilities|Array|Random (LocalVariables|GetCrates)))))
    (Actor|DestroyActor _output_get)
    (Utilities|Array|RemoveItem (LocalVariables|GetCrates) (LocalVariables|GetRandom%20Crate))))